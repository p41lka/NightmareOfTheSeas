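; Base NPC actor that shows its name in world text and lets players interact with it by proximity.
; On BeginPlay it sets a TextRender to the name supplied by its NPCManager.
; When a character begins or ends overlap, it casts that character's controller PlayerState to BP_MyPlayerState and calls StartNPCInteract with itself or StopNPCinteract.
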(event EventBeginPlay
  (Rendering|Components|TextRender|SetText (Variables|Default|GetTextRender) (Utilities|Text|ToText(String) (Class|NPCManager|GetNPCName (Variables|Default|GetNPCManager)))))

(event EventTick
  (params (DeltaSeconds :type Float%20%28single-precision%29)))

(event Collision|EventActorBeginOverlap
  (params (OtherActor :type Actor%20Object%20Reference))
  (bind _ascharacter (Utilities|Casting|CastToCharacter OtherActor))
  (bind _asbp_my_player_state (Utilities|Casting|CastToBP_MyPlayerState (Variables|/Script/Engine.Controller|GetPlayerState (Pawn|GetController _ascharacter))))
  (Default|StartNPCInteract _asbp_my_player_state self))

(event Collision|EventActorEndOverlap
  (params (OtherActor :type Actor%20Object%20Reference))
  (bind _ascharacter (Utilities|Casting|CastToCharacter OtherActor))
  (bind _asbp_my_player_state (Utilities|Casting|CastToBP_MyPlayerState (Variables|/Script/Engine.Controller|GetPlayerState (Pawn|GetController _ascharacter))))
  (Default|StopNPCinteract _asbp_my_player_state))

(fn ConstructionScript)