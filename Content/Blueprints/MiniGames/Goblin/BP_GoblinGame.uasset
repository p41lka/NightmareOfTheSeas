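; Potato-peeling minigame attached to the ship, with a blended camera switch, mouse input and a radial countdown widget.
; Each click swings the knife, rotates the potato and recolors one slice, with finished potatoes counted on the widget.
; Clicking beyond a periodically reset limit cuts the potato to a smaller mesh and remaps its slice progress.
; Timeout or too many cuts ends the game; Tick prints debug values.
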(event OnClicked(Potato)
  (params (TouchedComponent :type Primitive%20Component%20Object%20Reference) (ButtonPressed :type Key%20Structure :default "None"))
  ;[0 0 0] Click on potato
  (Audio|PlaySound2D "/Game/Sounds/C_Peel.C_Peel" 1.0 1.0 0.0 0 0)
  (Niagara|SpawnSystematLocation "/Game/VFXs/Peel/NS_Peel.NS_Peel" (Transformation|GetWorldLocation (Variables|Default|GetArrow_Particle)))
  (CallFunction|MoveKnife)
  (CallFunction|Rotate)
  (bind _result (Math|Integer|IncrementInt (Variables|Default|GetCurrentAllClicks))
    (:%20%20
      (if (<= _result (Variables|Default|GetMaxClicks))
        (if (>= (Variables|Default|GetCurrentSlice) (Utilities|Select :Index (Variables|Default|GetPotatoScale) :Option%200 0 :Option%201 9 :Option%202 7 :Option%203 5 :Option%204 4))
          (CallFunction|NewPotato)
          (bind _result_2 (Math|Integer|IncrementInt (Variables|Default|GetPotatoesPilled))
            (:%20%20
              (Variables|/Game/UI/Widgets/W_RadialTimer.W_RadialTimer_C|SetPotatoPeeled (Variables|Default|GetTimerWidget) _result_2)))
          (else
            (Math|Integer|IncrementInt (Variables|Default|GetCurrentSlice)
              (:%20%20
                (CallFunction|ChangeMaterial)))))
        (else
          (Math|Integer|IncrementInt (Variables|Default|GetCurrentSlice)
            (:%20%20
              (CallFunction|ChangeMaterial)
              (CallFunction|Cut))))))))

(event Custom|StartGame
  (bind _returnvalue (Transformation|GetActorLocation))
  (bind _returnvalue_2 (Game|GetPlayerController 0))
  (bind _charref (Variables|Default|GetCharREF))
  ;[0 0 0] Start and End minigame
  (Transformation|SetActorLocation _charref (Math|Vector|MakeVector (.x _returnvalue) (.y _returnvalue) (.z (Transformation|GetActorLocation _charref))) false true)
  (Game|Player|SetViewTargetwithBlend _returnvalue_2 self 0.7 "VTBlend_Linear" 0.0 false)
  (Input|SetInputModeGameandUI _returnvalue_2 0 "DoNotLock" false false)
  (Variables|/Script/Engine.PlayerController|SetbShowMouseCursor _returnvalue_2 true)
  (CallFunction|GameTimer)
  (Rendering|SetVisibility (Variables|Default|GetPotato) true false)
  (UserInterface|Viewport|AddtoViewport (Variables|Default|GetTimerWidget) 0)
  (CallFunction|StartPeelTimer))

(event Custom|EndGame
  (bind _returnvalue (Game|GetPlayerController 0))
  (bind _timerwidget (Variables|Default|GetTimerWidget))
  ;[0 0 0] Start and End minigame
  (Game|Player|SetViewTargetwithBlend (Game|GetPlayerController 0) (Variables|Default|GetCharREF) 0.7 "VTBlend_Linear" 0.0 false)
  (Default|ChangetoTPS (Variables|Default|GetCharREF) "NewEnumerator3")
  (Utilities|Time|ClearandInvalidateTimerbyHandle (Variables|Default|GetTimer))
  (Input|SetInputModeGameOnly _returnvalue false)
  (Variables|/Script/Engine.PlayerController|SetbShowMouseCursor _returnvalue false)
  (Rendering|SetVisibility (Variables|Default|GetKnife) false false)
  (Widget|RemovefromParent _timerwidget)
  (Variables|/Game/UI/Widgets/W_RadialTimer.W_RadialTimer_C|SetPercent _timerwidget 1.0)
  (bind _output_get (Variables|Default|SetPotatoesPilled 0))
  (Variables|/Game/UI/Widgets/W_RadialTimer.W_RadialTimer_C|SetPotatoPeeled (Variables|Default|GetTimerWidget) _output_get))

(event Custom|PeelTimer
  (Variables|Default|SetCurrentAllClicks 0))

(event Custom|SetNewRotation
  ;[1 1 1] Rotation
  (Transformation|SetRelativeRotation (Variables|Default|GetPotato) (Math|Rotator|MakeRotator 1.6e+02 9e+01 (* (/ 3.6e+02 (Utilities|Select :Index (Variables|Default|GetPotatoScale) :Option%200 0.0 :Option%201 1e+01 :Option%202 1e+01 :Option%203 8.0 :Option%204 5.0)) (Variables|Default|GetCurrentSlice))) false false))

(event Custom|SetNewSliceNumber
  (switch int (Variables|Default|GetPotatoScale)
    (:2
      (switch int (Variables|Default|GetCurrentSlice)
        (:0
          (Variables|Default|SetCurrentSlice 0))
        (:1
          (Variables|Default|SetCurrentSlice 1))
        (:2
          (Variables|Default|SetCurrentSlice 2 :!label _label))
        (:3
          (goto _label))
        (:4
          (Variables|Default|SetCurrentSlice 4 :!label _label_2))
        (:5
          (goto _label_2))
        (:6
          (Variables|Default|SetCurrentSlice 5))
        (:7
          (Variables|Default|SetCurrentSlice 6))
        (:8
          (Variables|Default|SetCurrentSlice 7 :!label _label_3))
        (:9
          (goto _label_3))))))

(event Custom|GameTimer
  ;[0 0 0] Timer
  (bind _returnvalue (Utilities|Time|SetTimerbyEvent (delegate Custom|MinusSec) 1.0 true))
  (Variables|Default|SetTimer _returnvalue))

(event Custom|MinusSec
  (bind _timerwidget (Variables|Default|GetTimerWidget))
  ;[0 0 0] Timer
  (bind _output_get (Variables|/Game/UI/Widgets/W_RadialTimer.W_RadialTimer_C|SetPercent _timerwidget (- (Variables|/Game/UI/Widgets/W_RadialTimer.W_RadialTimer_C|GetPercent _timerwidget) 0.05)))
  (Default|PercentFill _timerwidget (Variables|/Game/UI/Widgets/W_RadialTimer.W_RadialTimer_C|GetImage_0 _timerwidget) "/Game/UI/Widgets/M_RadialTimer.M_RadialTimer" _output_get)
  (if (<= _output_get 0.0)
    (CallFunction|NewPotato)
    (CallFunction|EndGame)))

(event Custom|Cut
  ;[0 0 0] Cut and change potato mesh
  (bind _result (Math|Integer|IncrementInt (Variables|Default|GetPotatoScale))
    (:%20%20
      (Variables|Default|SetCurrentAllClicks 0)
      (Components|StaticMesh|SetStaticMesh (Variables|Default|GetPotato) (Utilities|Select :Index _result :Option%200 "/Game/Meshes/MiniGames/SM_Potato_1.SM_Potato_1" :Option%201 "/Game/Meshes/MiniGames/SM_Potato_2.SM_Potato_2" :Option%202 "/Game/Meshes/MiniGames/SM_Potato_3.SM_Potato_3" :Option%203 "/Game/Meshes/MiniGames/SM_Potato_4.SM_Potato_4"))
      (CallFunction|SetNewSliceNumber)
      (CallFunction|SetNewRotation)
      (if (>= _result 4)
        ;;[1 1 1] game over
        (CallFunction|NewPotato)
        (CallFunction|EndGame)))))

(event Custom|MoveKnife
  (bind _alpha (Timeline|Timeline PlayFromStart)
    (:Update
      (Transformation|SetRelativeRotation (Variables|Default|GetKnife) (Math|Rotator|Lerp(Rotator) (Variables|Default|GetKnifeRotation) "-100.000000,90.000000,90.000000" _alpha true) false false))))

(event Custom|ChangeMaterial
  ;[0 0 0] Change material on peel
  (switch int (Variables|Default|GetPotatoScale)
    (:1
      _)
    (:2
      _)
    (:3
      _))
  (Rendering|Material|SetMaterial (Variables|Default|GetPotato) (Variables|Default|GetCurrentSlice) "/Game/Materials/Color/MI_Yellow.MI_Yellow"))

(event Custom|NewPotato
  (bind _potato (Variables|Default|GetPotato))
  ;[0 0 0] New Potato
  (Variables|Default|SetCurrentSlice 0)
  (Variables|Default|SetPotatoScale 1)
  (Components|StaticMesh|SetStaticMesh _potato "/Game/Meshes/MiniGames/SM_Potato_1.SM_Potato_1")
  (Transformation|SetRelativeRotation _potato "90.000000,0.000000,160.000000" false false)
  (for _index (range 0 (Rendering|Material|GetNumMaterials _potato))
    (Rendering|Material|SetMaterial _potato _index "/Game/Materials/Textured/Rana_Goblin_Stuff/MI_Potatos.MI_Potatos")))

(event Custom|Rotate
  ;[1 1 1] Rotation
  (Transformation|AddRelativeRotation (Variables|Default|GetPotato) (Math|Rotator|MakeRotator 0.0 0.0 (/ 3.6e+02 (Utilities|Select :Index (Variables|Default|GetPotatoScale) :Option%200 0.0 :Option%201 1e+01 :Option%202 1e+01 :Option%203 8.0 :Option%204 5.0))) false false))

(event Custom|StartPeelTimer
  (Utilities|Time|SetTimerbyEvent (delegate Custom|PeelTimer) 0.6 true))

(event EventBeginPlay
  (bind _knife (Variables|Default|GetKnife))
  (bind _asbp_third_person_character (Utilities|Casting|CastToBP_ThirdPersonCharacter (Game|GetPlayerCharacter 0)))
  (Variables|Default|SetCharREF _asbp_third_person_character)
  (Variables|Default|SetKnifeLocation (Variables|/Script/Engine.SceneComponent|GetRelativeLocation _knife))
  (Variables|Default|SetKnifeRotation (Variables|/Script/Engine.SceneComponent|GetRelativeRotation _knife))
  (bind _outactors (Actor|GetAllActorsOfClass "/Game/Blueprints/BP_Ship.BP_Ship_C"))
  (Transformation|AttachActorToActor (Utilities|Array|Get(acopy) _outactors) "None" "KeepWorld" "KeepWorld" "KeepWorld" true)
  (bind _returnvalue (UserInterface|CreateWidget "/Game/UI/Widgets/W_RadialTimer.W_RadialTimer_C"))
  (Variables|Default|SetTimerWidget _returnvalue))

(event EventTick
  (params (DeltaSeconds :type Float%20%28single-precision%29))
  (Development|PrintString (Utilities|String|ToString(Integer) (Variables|Default|GetCurrentSlice)) true true "(R=1.000000,G=0.000000,B=0.135502,A=1.000000)" 0.0)
  (Development|PrintString (Utilities|String|ToString(Integer) (Variables|Default|GetPotatoScale)) true true "(R=0.708678,G=0.433272,B=1.000000,A=1.000000)" 0.0))

(fn ConstructionScript)