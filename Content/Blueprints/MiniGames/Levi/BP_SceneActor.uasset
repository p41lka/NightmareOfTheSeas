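; BP_SceneActor is a moving hazard in the Levi minigame that damages the player and destroys itself on overlap.
; Each tick it steps 20 units backward along its Rotator component's forward vector, without delta-time scaling.
; It then copies the Rotator's world rotation from the Sphere of the first BP_EviromentMovement, so that sphere steers it.
; Any overlapping actor triggers the hit, since the handler casts player character 0 rather than checking OtherActor.
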(event Custom|OnActorBeginOverlap_Event
  (params (OverlappedActor :type Actor%20Object%20Reference) (OtherActor :type Actor%20Object%20Reference))
  (bind _asbp_third_person_character (Utilities|Casting|CastToBP_ThirdPersonCharacter (Game|GetPlayerCharacter 0)))
  (Default|RecieveDamage _asbp_third_person_character)
  (Actor|DestroyActor))

(event EventBeginPlay
  (bind _outactors (Actor|GetAllActorsOfClass "/Game/Blueprints/MiniGames/Levi/BP_EviromentMovement.BP_EviromentMovement_C"))
  (Variables|Default|SetEnvMove (Utilities|Array|Get(acopy) _outactors))
  (EventDispatchers|BindEventtoOnActorBeginOverlap (delegate Custom|OnActorBeginOverlap_Event)))

(event EventTick
  (params (DeltaSeconds :type Float%20%28single-precision%29))
  (bind _rotator (Variables|Default|Getrotator))
  (bind _returnvalue (Transformation|GetWorldLocation _rotator))
  (bind _returnvalue_2 (Math|Vector|GetForwardVector _rotator))
  (bind _returnvalue_3 (* _returnvalue_2 "-20.000000,-20.000000,-20.000000"))
  (Transformation|SetActorLocation (Math|Vector|MakeVector (+ (.x _returnvalue_3) (.x _returnvalue)) (+ (.y _returnvalue_3) (.y _returnvalue)) (+ (.z _returnvalue_3) (.z _returnvalue))) false false)
  (Transformation|SetWorldRotation (Variables|Default|Getrotator) (Transformation|GetWorldRotation (Variables|/Game/Blueprints/MiniGames/Levi/BP_EviromentMovement.BP_EviromentMovement_C|GetSphere (Variables|Default|GetEnvMove))) false false))

(fn ConstructionScript)