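; Stealth minigame actor that registers with the third-person character, where Rana digs to steal while avoiding being seen by patrolling Levi.
; Two timelines loop Levi between two points with idle pauses, and his overlap with the door collision sets the looking state.
; RanaStart cycles Rana through three positions until RanaEnd.
; Stealing while watched triggers EndGame, which returns the character to TPS and resets both characters.
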(event OnComponentBeginOverlap(DoorCollision)
  (params (OverlappedComponent :type Primitive%20Component%20Object%20Reference) (OtherActor :type Actor%20Object%20Reference) (OtherComp :type Primitive%20Component%20Object%20Reference) (OtherBodyIndex :type Integer) (bFromSweep :type Boolean) (SweepResult :type Hit%20Result%20Structure%20%28by%20ref%29))
  ;[0 0 0] Levi walks next to the door
  (if (== OtherComp (Variables|Default|GetLeviCollision))
    (Variables|Default|SetIsLooking true)
    (if (Variables|Default|GetIsStealing)
      (CallFunction|EndGame))))

(event OnComponentEndOverlap(DoorCollision)
  (params (OverlappedComponent :type Primitive%20Component%20Object%20Reference) (OtherActor :type Actor%20Object%20Reference) (OtherComp :type Primitive%20Component%20Object%20Reference) (OtherBodyIndex :type Integer))
  ;[0 0 0] Levi walks next to the door
  (if (== OtherComp (Variables|Default|GetLeviCollision))
    (Variables|Default|SetIsLooking false)))

(event Custom|RunLevi
  (bind _levi (Variables|Default|GetLevi))
  (bind _levi_2 (Variables|Default|GetLevi))
  (Transformation|SetRelativeRotation _levi "0.000000,90.000000,0.000000" false false :!label _label)
  (Components|Animation|PlayAnimation _levi "/Game/Animations/Mixamo/Levi/Walk.Walk" true)
  (bind _alpha (Timeline|Timeline PlayFromStart)
    (:Update
      (Transformation|SetRelativeLocation (Variables|Default|GetLeviCollision) (Math|Vector|Lerp(Vector) (Variables|Default|GetLeviPointA) (Variables|Default|GetLeviPointB) _alpha) false false))
    (:Finished
      (Components|Animation|PlayAnimation (Variables|Default|GetLevi) "/Game/Animations/Mixamo/Levi/Idle.Idle" true)
      (Utilities|FlowControl|Delay 2.0)
      (Transformation|SetRelativeRotation _levi_2 "0.000000,-90.000000,0.000000" false false)
      (Components|Animation|PlayAnimation _levi_2 "/Game/Animations/Mixamo/Levi/Walk.Walk" true)
      (bind _alpha_2 (Timeline|Timeline_0 PlayFromStart)
        (:Update
          (Transformation|SetRelativeLocation (Variables|Default|GetLeviCollision) (Math|Vector|Lerp(Vector) (Variables|Default|GetLeviPointB) (Variables|Default|GetLeviPointA) _alpha_2) false false))
        (:Finished
          (Components|Animation|PlayAnimation (Variables|Default|GetLevi) "/Game/Animations/Mixamo/Levi/Idle.Idle" true)
          (Utilities|FlowControl|Delay 2.0)
          (goto _label))))))

(event Custom|StartGame
  (CallFunction|FixCamera)
  (CallFunction|RunLevi))

(event Custom|FixCamera
  (bind _returnvalue (Game|GetPlayerCharacter 0))
  (bind _sphere (Variables|Default|GetSphere))
  (bind _returnvalue_2 (Transformation|GetWorldLocation _sphere))
  (Transformation|SetActorLocation _returnvalue (Math|Vector|MakeVector (.x _returnvalue_2) (.y _returnvalue_2) (.z (Transformation|GetActorLocation _returnvalue))) false false))

(event Custom|RanaStart
  (if (Variables|Default|GetIsLooking)
    (CallFunction|EndGame)
    (else
      (Components|Animation|PlayAnimation (Variables|Default|GetRana) "/Game/Animations/Mixamo/Rana/Dig.Dig" true)
      (bind _output_get (Variables|Default|SetIsStealing true))
      (if _output_get :!label _label
        (Transformation|SetRelativeLocation (Variables|Default|GetRana) (Variables|/Script/Engine.SceneComponent|GetRelativeLocation (Variables|Default|GetRana_1)) false false)
        (Utilities|FlowControl|Delay 0.5)
        (if (Variables|Default|GetIsStealing)
          (Transformation|SetRelativeLocation (Variables|Default|GetRana) (Variables|/Script/Engine.SceneComponent|GetRelativeLocation (Variables|Default|GetRana_2)) false false)
          (Utilities|FlowControl|Delay 0.5)
          (if (Variables|Default|GetIsStealing)
            (Transformation|SetRelativeLocation (Variables|Default|GetRana) (Variables|/Script/Engine.SceneComponent|GetRelativeLocation (Variables|Default|GetRana_3)) false false)
            (Utilities|FlowControl|Delay 0.5)
            (goto _label)))))))

(event Custom|RanaEnd
  (bind _rana (Variables|Default|GetRana))
  (Components|Animation|PlayAnimation _rana "/Game/Animations/Mixamo/Rana/Idle.Idle" true)
  (Transformation|SetRelativeLocation _rana "0.000000,270.000000,0.000000" false false)
  (Variables|Default|SetIsStealing false))

(event Custom|EndGame
  (Default|ChangetoTPS (Variables|Default|GetCharREf) "NewEnumerator2")
  (Audio|Components|Audio|Stop (Variables|Default|GetTimeline_0))
  (Audio|Components|Audio|Stop (Variables|Default|GetTimeline))
  (Transformation|SetRelativeLocation (Variables|Default|GetLeviCollision) "0.000000,0.000000,180.000000" false false)
  (Components|Animation|PlayAnimation (Variables|Default|GetLevi) "/Game/Animations/Mixamo/Levi/Idle.Idle" true)
  (CallFunction|RanaEnd))

(event EventBeginPlay
  (bind _asbp_third_person_character (Utilities|Casting|CastToBP_ThirdPersonCharacter (Game|GetPlayerCharacter 0)))
  (Variables|/Game/ThirdPerson/Blueprints/BP_ThirdPersonCharacter.BP_ThirdPersonCharacter_C|SetRanaGame _asbp_third_person_character self)
  (Variables|Default|SetCharREf _asbp_third_person_character))

(fn ConstructionScript)