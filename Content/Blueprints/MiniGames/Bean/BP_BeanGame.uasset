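; BP_BeanGame is a mini-game that scatters puddle spots over the ship and ends once all are cleared.
; StartGame traces down from random points in its Box to spawn randomly sized and rotated BP_Spot actors, attached to BP_Ship with a back-reference to the game.
; MinusSpot decrements the remaining count and, at zero, calls ChangeToTPS on the player character after a short delay.
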(event Custom|StartGame
  (bind _returnvalue (Transformation|GetActorLocation))
  (bind _box (Variables|Default|GetBox))
  (bind (_origin _boxextent) (Collision|GetComponentBounds _box))
  (bind _returnvalue_2 (Math|Random|RandomPointinBoundingBox _origin _boxextent))
  (bind _returnvalue_3 (Math|Transform|MakeTransform (Math|Vector|MakeVector (.x _returnvalue_2) (.y _returnvalue_2) (.z _returnvalue))))
  (Variables|Default|SetCurrentSpots (Variables|Default|GetMaxSpots))
  (for _index (range 1 (Variables|Default|GetMaxSpots))
    (bind _outhit (Collision|LineTraceByChannel (.location _returnvalue_3) (+ (.location _returnvalue_3) (* (Math|Vector|GetUpVector _box) -3e+02)) "TraceTypeQuery1" false 0 "None"))
    (bind _output_get (Variables|Default|SetPuddleSize (Math|Random|RandomFloatinRange 0.8 1.5)))
    (bind _returnvalue_4 (Game|SpawnActorfromClass "/Game/Blueprints/MiniGames/Bean/BP_Spot.BP_Spot_C" (Math|Transform|MakeTransform (.Location (Collision|BreakHitResult _outhit)) "0, 0, 0" (Math|Vector|MakeVector 1.0 _output_get _output_get)) "Undefined" "MultiplyWithRoot" 0 0))
    (Transformation|AttachActorToActor _returnvalue_4 (Variables|Default|GetShip) "None" "KeepWorld" "SnapToTarget" "KeepWorld" false)
    (Variables|/Game/Blueprints/MiniGames/Bean/BP_Spot.BP_Spot_C|SetBinGame _returnvalue_4 self)
    (Transformation|SetActorRotation _returnvalue_4 (Math|Rotator|MakeRotator (.roll (Transformation|GetActorRotation _returnvalue_4)) (.pitch (Transformation|GetActorRotation _returnvalue_4)) (Math|Random|RandomFloatinRange 0.0 3.6e+02)))))

(event Custom|MinusSpot
  (bind _result (Math|Integer|DecrementInt (Variables|Default|GetCurrentSpots))
    (:%20%20
      (if (<= _result 0)
        (Utilities|FlowControl|Delay 0.2)
        (bind _asbp_third_person_character (Utilities|Casting|CastToBP_ThirdPersonCharacter (Game|GetPlayerCharacter 0)))
        (Default|ChangetoTPS _asbp_third_person_character "NewEnumerator0")))))

(event EventBeginPlay
  (bind _outactors (Actor|GetAllActorsOfClass "/Game/Blueprints/BP_Ship.BP_Ship_C"))
  (Variables|Default|SetShip (Utilities|Array|Get(acopy) _outactors)))

(fn ConstructionScript)