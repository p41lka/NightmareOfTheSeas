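; A paint spot decal actor for the Bean minigame that is cleaned by mopping.
; On BeginPlay it creates a dynamic decal material and randomizes its color and paint texture.
; Each Mop event decrements Dirtiness, fading the decal when one level remains.
; At zero it reports the removed spot to BinGame through MinusSpot and destroys itself.
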(event EventBeginPlay
  (bind _returnvalue (Rendering|Material|CreateDynamicMaterialInstance (Variables|Default|GetDecal) :!class /Script/Engine.DecalComponent))
  (bind _output_get (Variables|Default|SetDecalMaterial _returnvalue))
  (Rendering|Material|SetVectorParameterValue _output_get "Color" (Utilities|Select :Index (Math|Random|RandomIntegerinRange 0 5) :Option%200 "(R=0.616667,G=0.131701,B=0.339836,A=1.000000)" :Option%201 "(R=0.000000,G=0.340000,B=1.000000,A=1.000000)" :Option%202 "(R=1.000000,G=0.048555,B=0.024679,A=1.000000)" :Option%203 "(R=1.000000,G=0.770315,B=0.000000,A=1.000000)" :Option%204 "(R=0.077228,G=0.766667,B=0.106093,A=1.000000)" :Option%205 "(R=0.336171,G=0.000000,B=0.925000,A=1.000000)") :!class /Script/Engine.MaterialInstanceDynamic)
  (Rendering|Material|SetTextureParameterValue _output_get "Texture" (Utilities|Select :Index (Math|Random|RandomIntegerinRange 0 2) :Option%200 "/Game/Materials/Decals/Paint1.Paint1" :Option%201 "/Game/Materials/Decals/Paint2.Paint2" :Option%202 "/Game/Materials/Decals/Paint3.Paint3")))

(event EventMop
  (bind _result (Math|Integer|DecrementInt (Variables|Default|GetDirtiness))
    (:%20%20
      (switch int _result
        (:0
          (Default|MinusSpot (Variables|Default|GetBinGame))
          (Actor|DestroyActor))
        (:1
          (Rendering|Material|SetScalarParameterValue (Variables|Default|GetDecalMaterial) "Opacity" 0.3 :!class /Script/Engine.MaterialInstanceDynamic))))))

(fn ConstructionScript)