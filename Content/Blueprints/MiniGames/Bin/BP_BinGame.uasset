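; BP_BinGame is the manager actor for the bin mini-game, in which a set number of spots must be used up.
; StartGame spawns MaxSpots BP_Spot actors at random XY points within the Box bounds, at the actor's height, each holding a reference back to it.
; MinusSpot counts the spots down; at zero it waits briefly, then calls ChangeToTPS on the player's BP_ThirdPersonCharacter.
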(event Custom|StartGame
  (bind _box (Variables|Default|GetBox))
  (bind (_origin _boxextent) (Collision|GetComponentBounds _box))
  (bind _returnvalue (Math|Random|RandomPointinBoundingBox _origin _boxextent))
  (Variables|Default|SetCurrentSpots (Variables|Default|GetMaxSpots))
  (for _index (range 1 (Variables|Default|GetMaxSpots))
    (bind _returnvalue_2 (Game|SpawnActorfromClass "/Game/Blueprints/MiniGames/Bin/BP_Spot.BP_Spot_C" (Math|Transform|MakeTransform (Math|Vector|MakeVector (.x _returnvalue) (.y _returnvalue) (.z (Transformation|GetActorLocation))) "0, 0, 0" "1.000000,1.000000,1.000000") "Undefined" "MultiplyWithRoot" 0 0))
    (Variables|/Game/Blueprints/MiniGames/Bin/BP_Spot.BP_Spot_C|SetBinGame _returnvalue_2 self)))

(event Custom|MinusSpot
  (bind _result (Math|Integer|DecrementInt (Variables|Default|GetCurrentSpots))
    (:%20%20
      (if (<= _result 0)
        (Utilities|FlowControl|Delay 0.2)
        (bind _asbp_third_person_character (Utilities|Casting|CastToBP_ThirdPersonCharacter (Game|GetPlayerCharacter 0)))
        (Default|ChangetoTPS _asbp_third_person_character)))))

(event EventBeginPlay)

(fn ConstructionScript)