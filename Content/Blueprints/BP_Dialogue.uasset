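; BP_Dialogue is an interactable actor that opens a dialogue UI for the first player.
; Interact creates a W_Dialogue widget, passes itself to it, then StartDialogue shows it, disables character movement and switches to UI-only input with a cursor.
; EndDialogue removes the widget and restores walking and game-only input.
; StartEvent ends the dialogue and prints a placeholder event message.
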(event Custom|StartDialogue
  (bind _returnvalue (Game|GetPlayerController 0))
  (UserInterface|Viewport|AddtoViewport (Variables|Default|GetDialogueWidget) 0)
  (Pawn|Components|CharacterMovement|DisableMovement (Variables|/Script/Engine.Character|GetCharacterMovement (Game|GetPlayerCharacter 0)))
  (Input|SetInputModeUIOnly _returnvalue 0 "DoNotLock" false)
  (Variables|/Script/Engine.PlayerController|SetbShowMouseCursor _returnvalue true))

(event Custom|EndDialogue
  (bind _returnvalue (Game|GetPlayerController 0))
  (Widget|RemovefromParent (Variables|Default|GetDialogueWidget))
  (Pawn|Components|CharacterMovement|SetMovementMode (Variables|/Script/Engine.Character|GetCharacterMovement (Game|GetPlayerCharacter 0)) "MOVE_Walking" 0)
  (Input|SetInputModeGameOnly _returnvalue false)
  (Variables|/Script/Engine.PlayerController|SetbShowMouseCursor _returnvalue false))

(event Custom|StartEvent
  (CallFunction|EndDialogue)
  (Development|PrintString "СОБЫТИЕ!!!"))

(event EventBeginPlay
  (|CallParentFunction) ; This node is disabled and will not be called.\nDrag off pins to build functionality.
)

(event Collision|EventActorBeginOverlap
  (params (OtherActor :type Actor%20Object%20Reference))
  (|CallParentFunction OtherActor) ; This node is disabled and will not be called.\nDrag off pins to build functionality.
)

(event EventTick
  (params (DeltaSeconds :type Float%20%28single-precision%29))
  (|CallParentFunction DeltaSeconds) ; This node is disabled and will not be called.\nDrag off pins to build functionality.
)

(event EventInteract
  (|CallParentFunction)
  (bind _returnvalue (UserInterface|CreateWidget "/Game/UI/Widgets/W_Dialogue.W_Dialogue_C" (Game|GetPlayerController 0)))
  (bind _output_get (Variables|Default|SetDialogueWidget _returnvalue))
  (Default|SetDialogue _output_get self)
  (CallFunction|StartDialogue))

(fn ConstructionScript
  (|CallParentFunction))