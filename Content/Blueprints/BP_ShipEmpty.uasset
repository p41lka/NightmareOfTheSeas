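; BP_ShipEmpty is a ship actor that rocks with small random pitch and roll to simulate waves.
; Waves picks random tilts within about a degree and alternates branches via IsInverting, though PreviousRot is re-rolled each call before its modified values are used.
; WavesTurn plays TimelineWaves to lerp roll and pitch to that target, while yaw follows the EnvMove Sphere's world rotation.
; Nothing in this file calls Waves.
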(event Custom|WavesTurn
  (params (RotInit :type Rotator) (Rot :type Rotator))
  (bind _alpha (Timeline|TimelineWaves PlayFromStart)
    (:Update
      (Transformation|SetActorRotation (Math|Rotator|MakeRotator (.Roll (Math|Rotator|BreakRotator (Math|Rotator|Lerp(Rotator) RotInit Rot _alpha true))) (.Pitch (Math|Rotator|BreakRotator (Math|Rotator|Lerp(Rotator) RotInit Rot _alpha true))) (.yaw (Transformation|GetWorldRotation (Variables|/Game/Blueprints/MiniGames/Levi/BP_EviromentMovement.BP_EviromentMovement_C|GetSphere (Variables|Default|GetEnvMove)))))))))

(fn ConstructionScript)

(fn Waves
  (bind _returnvalue (Math|Random|RandomIntegerinRange -1 1))
  (bind _returnvalue_2 (Math|Random|RandomIntegerinRange 1 -1))
  (bind _returnvalue_3 (Math|Conversions|ToFloat(Integer) _returnvalue_2))
  (bind _returnvalue_4 (Math|Conversions|ToFloat(Integer) _returnvalue))
  (bind _returnvalue_5 (Math|Rotator|MakeRotator _returnvalue_3 _returnvalue_4 0.0))
  (Variables|Default|SetPreviousRot _returnvalue_5)
  (if (Variables|Default|GetIsInverting)
    (bind _result (Math|Float|NegateFloat (.roll (Variables|Default|GetPreviousRot)))
      (:%20%20
        (bind _result_2 (Math|Float|NegateFloat (.pitch (Variables|Default|GetPreviousRot)))
          (:%20%20
            (CallFunction|WavesTurn (Transformation|GetActorRotation) (Math|Rotator|MakeRotator _result _result_2 (.yaw (Variables|Default|GetPreviousRot))))
            (Variables|Default|SetIsInverting false)))))
    (else
      (CallFunction|WavesTurn (Transformation|GetActorRotation) _returnvalue_5)
      (Variables|Default|SetIsInverting true))))