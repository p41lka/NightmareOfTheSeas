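; Light manager that switches the level's lighting between Day and Evening once the player QuestLogComponent's gamemode timer reaches a threshold.
; BeginPlay applies the current time's parameter maps to directional light, fog and sky sphere, then polls every second until one change triggers.
; A Timeline, played forward or reversed, blends intensity, sun rotation, fog density and sun height.
; On finish it snaps colors, flips Time and updates the Ship's sound.
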(event Custom|CheckTime
  (if (>= (Variables|/Game/Defender/Blueprints/Components/QuestLogComponent.QuestLogComponent_C|GetGamemodeTimer (Variables|Default|GetQuest%20Log%20Comp)) (Variables|Default|GetTimeForChange))
    (CallFunction|ChangeParams (Variables|Default|GetTime))
    (Utilities|Time|ClearandInvalidateTimerbyHandle (Variables|Default|GetTimer))))

(event Custom|ChangeParams
  (params (Time :type E_DayTime%20Enum :default "NewEnumerator0"))
  (bind _directlightparams (Variables|Default|GetDirectLightParams))
  (bind _directlight (Variables|Default|GetDirectLight))
  (bind _ship (Variables|Default|GetShip))
  (bind _directlightparams_2 (Variables|Default|GetDirectLightParams))
  (bind _exponentialfogparams (Variables|Default|GetExponentialFogParams))
  (bind _exponentialfogparams_2 (Variables|Default|GetExponentialFogParams))
  (bind _directlight_2 (Variables|Default|GetDirectLight))
  (bind _exponentialfog (Variables|Default|GetExponentialFog))
  (bind _skysphere (Variables|Default|GetSkySphere))
  (bind _value (Utilities|Map|Find _exponentialfogparams "NewEnumerator1"))
  (bind _value_2 (Utilities|Map|Find _directlightparams "NewEnumerator0"))
  (bind _value_3 (Utilities|Map|Find _directlightparams_2 "NewEnumerator1"))
  (bind _value_4 (Utilities|Map|Find _exponentialfogparams_2 "NewEnumerator0"))
  (bind _lightcomponent (Variables|/Script/Engine.Light|GetLightComponent _directlight_2))
  (bind _component (Variables|/Script/Engine.ExponentialHeightFog|GetComponent _exponentialfog))
  (bind (_intensity _color) (Utilities|Struct|BreakS_LightParams _value))
  (bind (_intensity_2 _color_2) (Utilities|Struct|BreakS_LightParams _value_4))
  (bind (_intensity_3 _rotation _color_3) (Utilities|Struct|BreakS_LightParams _value_2))
  (bind (_intensity_4 _rotation_2 _color_4) (Utilities|Struct|BreakS_LightParams _value_3))
  (switch Utilities|FlowControl|Switch|SwitchonE_DayTime Time
    (:NewEnumerator0
      (bind _alpha (Timeline|Timeline PlayFromStart)
        (:Update
          (Rendering|Components|Light|SetIntensity (Variables|/Script/Engine.Light|GetLightComponent _directlight) (Math|Float|Lerp _intensity_3 _intensity_4 _alpha))
          (Transformation|SetActorRotation _directlight (Math|Rotator|Lerp(Rotator) _rotation _rotation_2 _alpha true))
          (Class|ExponentialHeightFogComponent|SetFogDensity (Variables|/Script/Engine.ExponentialHeightFog|GetComponent (Variables|Default|GetExponentialFog)) (Math|Float|Lerp _intensity_2 _intensity _alpha))
          (Variables|/Game/DreamscapeSeries/SharedResources/CUSTOMSKY/BP_Sky_Sphere_Stylized1.BP_Sky_Sphere_Stylized1_C|SetSun%20height _skysphere (Math|Float|Lerp (Utilities|Struct|BreakS_LightParams (.Value (Utilities|Map|Find (Variables|Default|GetSkySphereParams) "NewEnumerator0"))) (Utilities|Struct|BreakS_LightParams (.Value (Utilities|Map|Find (Variables|Default|GetSkySphereParams) "NewEnumerator1"))) _alpha))
          (Default|RefreshMaterial _skysphere))
        (:Finished
          (switch Utilities|FlowControl|Switch|SwitchonE_DayTime (Variables|Default|GetTime)
            (:NewEnumerator0
              (Rendering|Components|Light|SetLightColor _lightcomponent (Math|Conversions|ToLinearColor(Color) _color_4) true)
              (Class|ExponentialHeightFogComponent|SetFogInscatteringColor _component (Math|Conversions|ToLinearColor(Color) _color))
              (bind _output_get (Variables|Default|SetTime "NewEnumerator1"))
              (Utilities|IsValid _ship
                (:Is%20Valid
                  (Default|ChangeSound _ship _output_get))))
            (:NewEnumerator1
              (Rendering|Components|Light|SetLightColor _lightcomponent (Math|Conversions|ToLinearColor(Color) _color_3) true)
              (Class|ExponentialHeightFogComponent|SetFogInscatteringColor _component (Math|Conversions|ToLinearColor(Color) _color_2))
              (bind _output_get_2 (Variables|Default|SetTime "NewEnumerator0"))
              (Utilities|IsValid _ship
                (:Is%20Valid
                  (Default|ChangeSound _ship _output_get_2))))))))
    (:NewEnumerator1
      (Timeline|Timeline ReverseFromEnd))))

(event EventBeginPlay
  (CallFunction|SetParamfromTime (Variables|Default|GetTime))
  (bind _asbp_third_person_character (Utilities|Casting|CastToBP_ThirdPersonCharacter (Game|GetPlayerCharacter 0)))
  (Variables|Default|SetQuest%20Log%20Comp (Variables|/Game/ThirdPerson/Blueprints/BP_ThirdPersonCharacter.BP_ThirdPersonCharacter_C|GetQuestLogComponent _asbp_third_person_character))
  (bind _returnvalue (Utilities|Time|SetTimerbyEvent (delegate Custom|CheckTime) 1.0 true))
  (Variables|Default|SetTimer _returnvalue))

(fn ConstructionScript)

(fn SetParamfromTime
  (params (Time :type E_DayTime%20Enum :default "NewEnumerator0"))
  (CallFunction|SetParams (.Value (Utilities|Map|Find (Variables|Default|GetDirectLightParams) Time)) (.Value (Utilities|Map|Find (Variables|Default|GetExponentialFogParams) Time)) (.Value (Utilities|Map|Find (Variables|Default|GetSkySphereParams) Time))))

(fn SetParams
  (params (DirectLight :type S%20Light%20Params%20Structure) (ExponentialFog :type S%20Light%20Params%20Structure) (NewParam :type S%20Light%20Params%20Structure))
  (bind (_intensity _rotation _color) (Utilities|Struct|BreakS_LightParams DirectLight))
  (bind (_intensity_2 _rotation_2 _color_2) (Utilities|Struct|BreakS_LightParams ExponentialFog))
  (bind _skysphere (Variables|Default|GetSkySphere))
  (bind _lightcomponent (Variables|/Script/Engine.Light|GetLightComponent (Variables|Default|GetDirectLight)))
  (bind _component (Variables|/Script/Engine.ExponentialHeightFog|GetComponent (Variables|Default|GetExponentialFog)))
  (Rendering|Components|Light|SetIntensity _lightcomponent _intensity)
  (Transformation|SetActorRotation (Variables|Default|GetDirectLight) _rotation)
  (Rendering|Components|Light|SetLightColor _lightcomponent (Math|Conversions|ToLinearColor(Color) _color) true)
  (Class|ExponentialHeightFogComponent|SetFogDensity _component _intensity_2)
  (Class|ExponentialHeightFogComponent|SetFogInscatteringColor _component (Math|Conversions|ToLinearColor(Color) _color_2))
  (Variables|/Game/DreamscapeSeries/SharedResources/CUSTOMSKY/BP_Sky_Sphere_Stylized1.BP_Sky_Sphere_Stylized1_C|SetSun%20height _skysphere (.Intensity (Utilities|Struct|BreakS_LightParams NewParam)))
  (Default|RefreshMaterial _skysphere))