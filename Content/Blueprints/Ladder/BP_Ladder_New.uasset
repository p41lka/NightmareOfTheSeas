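; Procedural ladder actor that builds itself to a set Height and tells overlapping actors which ladder they are at.
; The construction script moves LadderTop to Height, stretches both side rails and the collider to fit, then adds randomly chosen step meshes every CrossbarGap.
; Collider begin overlap sends the ladder to the other actor through SetLadderMessage, and end overlap sends an empty reference.
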(event OnComponentBeginOverlap(LadderCollider)
  (params (OverlappedComponent :type Primitive%20Component%20Object%20Reference) (OtherActor :type Actor%20Object%20Reference) (OtherComp :type Primitive%20Component%20Object%20Reference) (OtherBodyIndex :type Integer) (bFromSweep :type Boolean) (SweepResult :type Hit%20Result%20Structure%20%28by%20ref%29))
  (Class|BPClimber|SetLadder(Message) OtherActor self))

(event OnComponentEndOverlap(LadderCollider)
  (params (OverlappedComponent :type Primitive%20Component%20Object%20Reference) (OtherActor :type Actor%20Object%20Reference) (OtherComp :type Primitive%20Component%20Object%20Reference) (OtherBodyIndex :type Integer))
  (Class|BPClimber|SetLadder(Message) OtherActor))

(event Custom|InitLadder
  (Transformation|SetRelativeLocation (Variables|Default|GetLadderTop) (Math|Vector|MakeVector 0.0 0.0 (Variables|Default|GetHeight)) false false)
  (Utilities|AdjustSideBar (Variables|Default|GetLadder_L))
  (Utilities|AdjustSideBar (Variables|Default|GetLadder_R))
  (Utilities|AdjustSideBar (Variables|Default|GetLadderCollider))
  (Variables|Default|SetTemp_Height 0.0)
  (Utilities|Array|Clear (Variables|Default|GetSteps_1))
  (while (< (Variables|Default|GetTemp_Height) (.z (Variables|/Script/Engine.SceneComponent|GetRelativeLocation (Variables|Default|GetLadderTop))))
    (bind _returnvalue (AddComponent|AddStaticMeshComponent false (Math|Transform|MakeTransform (Math|Vector|MakeVector 0.0 0.0 (Variables|Default|GetTemp_Height)) "0.000000,90.000000,0.000000" "1.500000,1.500000,1.500000")))
    (Utilities|Array|Add (Variables|Default|GetSteps_1) _returnvalue)
    (Components|StaticMesh|SetStaticMesh _returnvalue (.OutItem (Utilities|Array|Random (Variables|Default|GetSteps))))
    (Variables|Default|SetTemp_Height (+ (Variables|Default|GetTemp_Height) (Variables|Default|GetCrossbarGap)))))

(fn ConstructionScript
  (CallFunction|InitLadder))