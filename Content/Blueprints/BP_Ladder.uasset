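; BP_Ladder is a climbable ladder actor that switches the third-person character into a climbing state when it enters the ladder's trigger box.
; Entering the box sets flying movement, zeroes velocity, snaps the character to the Arrow's XY facing opposite the ladder's yaw, and attaches it.
; Leaving detaches the character and restores walking, then briefly disables the box's overlap events to prevent an immediate re-grab.
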(event OnComponentBeginOverlap(Box)
  (params (OverlappedComponent :type Primitive%20Component%20Object%20Reference) (OtherActor :type Actor%20Object%20Reference) (OtherComp :type Primitive%20Component%20Object%20Reference) (OtherBodyIndex :type Integer) (bFromSweep :type Boolean) (SweepResult :type Hit%20Result%20Structure%20%28by%20ref%29))
  (bind _asbp_third_person_character (Utilities|Casting|CastToBP_ThirdPersonCharacter OtherActor))
  (bind _output_get (Variables|Default|SetCharREF _asbp_third_person_character))
  (if (not (Variables|/Game/ThirdPerson/Blueprints/BP_ThirdPersonCharacter.BP_ThirdPersonCharacter_C|GetOnLadder _output_get))
    (CallFunction|GrabLadder)))

(event OnComponentEndOverlap(Box)
  (params (OverlappedComponent :type Primitive%20Component%20Object%20Reference) (OtherActor :type Actor%20Object%20Reference) (OtherComp :type Primitive%20Component%20Object%20Reference) (OtherBodyIndex :type Integer))
  (bind _asbp_third_person_character (Utilities|Casting|CastToBP_ThirdPersonCharacter OtherActor))
  (if (Variables|/Game/ThirdPerson/Blueprints/BP_ThirdPersonCharacter.BP_ThirdPersonCharacter_C|GetOnLadder _asbp_third_person_character)
    (CallFunction|ExitLadder)))

(event Custom|GrabLadder
  (bind _returnvalue (Transformation|GetActorRotation))
  (bind _charref (Variables|Default|GetCharREF))
  (bind _arrow (Variables|Default|GetArrow))
  (bind _charref_2 (Variables|Default|GetCharREF))
  (bind _returnvalue_2 (Transformation|GetWorldLocation _arrow))
  (bind _returnvalue_3 (- (.yaw _returnvalue) 1.8e+02))
  (bind _charactermovement (Variables|/Script/Engine.Character|GetCharacterMovement _charref_2))
  (Variables|/Game/ThirdPerson/Blueprints/BP_ThirdPersonCharacter.BP_ThirdPersonCharacter_C|SetOnLadder _charref_2 true)
  (Variables|/Game/ThirdPerson/Blueprints/BP_ThirdPersonCharacter.BP_ThirdPersonCharacter_C|SetState _charref_2 "NewEnumerator1")
  (Pawn|Components|CharacterMovement|SetMovementMode _charactermovement "MOVE_Flying" 0)
  (Variables|/Script/Engine.MovementComponent|SetVelocity _charactermovement "0, 0, 0")
  (Transformation|SetActorLocationAndRotation _charref_2 (Math|Vector|MakeVector (.x _returnvalue_2) (.y _returnvalue_2) (.z (Transformation|GetActorLocation _charref_2))) (Math|Rotator|MakeRotator 0.0 0.0 _returnvalue_3))
  (Transformation|AttachActorToActor _charref self "None" "KeepWorld" "KeepWorld" "KeepWorld" true)
  (Variables|/Game/ThirdPerson/Blueprints/BP_ThirdPersonCharacter.BP_ThirdPersonCharacter_C|SetLadderRotation _charref _returnvalue_3))

(event Custom|ExitLadder
  (bind _box (Variables|Default|GetBox))
  (bind _charref (Variables|Default|GetCharREF))
  (Variables|/Game/ThirdPerson/Blueprints/BP_ThirdPersonCharacter.BP_ThirdPersonCharacter_C|SetOnLadder _charref false)
  (Transformation|DetachFromActor _charref "KeepWorld" "KeepWorld" "KeepWorld")
  (Variables|/Game/ThirdPerson/Blueprints/BP_ThirdPersonCharacter.BP_ThirdPersonCharacter_C|SetState _charref "NewEnumerator0")
  (Pawn|Components|CharacterMovement|SetMovementMode (Variables|/Script/Engine.Character|GetCharacterMovement _charref) "MOVE_Walking" 0)
  (Development|PrintString "exit")
  (Variables|/Script/Engine.PrimitiveComponent|SetbGenerateOverlapEvents _box false)
  (Utilities|FlowControl|Delay 0.5)
  (Variables|/Script/Engine.PrimitiveComponent|SetbGenerateOverlapEvents _box true))

(fn ConstructionScript)