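; BP_BaseQuestTask is a base Blueprint for quest tasks in the quest editor system, defining common functions that describe a task.
; It supplies defaults for color, name, short description and timer, plus flags that enable announcing and UI display.
; Each function only returns a constant, with the short description ignoring its payload inputs, so the graphs hold no quest logic.
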(fn GetTaskColor
  (return ""))

(fn GetTaskName
  (return ""))

(fn GetTaskShortDescription
  (params (PayloadIn :type Quest%20Task%20Payload%20Structure%20%28by%20ref%29) (CustomPayloadDataIn :type Array%20of%20Strings))
  (return ""))

(fn GetTaskTimer
  (return 0.0))

(fn TaskShouldAnnounce
  (return true))

(fn TaskShouldShowinUI
  (return true))