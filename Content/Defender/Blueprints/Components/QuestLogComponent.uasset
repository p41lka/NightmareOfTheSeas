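; Quest log component that spawns a BP_QuestParent per quest, tracks active and completed quests, and shows completion or failure messages.
; Quests start from dialogue events, chained rewards or a per-second gamemode timer that fires timed quests and events from DataTables, pausing while dialogue is visible.
; Turn-in adds success or FailReward items to the player's inventory.
; Name substrings like GiveQuest, QuestObjective, NextQuest and ExecuteEvent act as commands in dialogue and rewards.
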(event Custom|GiveQuest
  (params (FunctionName :type Name))
  (bind _returnvalue (Utilities|String|ToString(Name) FunctionName))
  (if (Utilities|String|Contains _returnvalue "GiveQuest")
    (if (Utilities|String|Contains _returnvalue "QuestObjective")
      (Default|CallObjectIDPassed (Variables|Default|GetInteractorConponent) (Utilities|String|StringToName (Utilities|String|Replace _returnvalue "QuestObjective")) 1)
      (elif true
        (CallFunction|AddNewQuest (Utilities|String|StringToName (Utilities|String|Replace _returnvalue "GiveQuest")))))))

(event EventBeginPlay
  (bind _returnvalue (Game|GetPlayerCharacter 0))
  (bind _returnvalue_2 (Actor|GetComponentbyClass _returnvalue "/Game/Defender/Blueprints/Components/InteractorComp.InteractorComp_C"))
  (Utilities|IsValid _returnvalue_2
    (:Is%20Valid
      (Variables|Default|SetInteractorConponent _returnvalue_2)
      (bind _returnvalue_3 (Game|ConstructObjectfromClass "/Game/Defender/Blueprints/WidgetBP/WB_GamemodeTimer.WB_GamemodeTimer_C" self))
      (UserInterface|Viewport|AddtoViewport _returnvalue_3 0)
      (bind _returnvalue_4 (Utilities|Time|SetTimerbyFunctionName 0 "AutoQuestAndEventGamemodeTimer" 1.0 true))
      (Variables|Default|SetTimerHandle _returnvalue_4)
      (bind _outactors (Actor|GetAllActorsOfClass "/Game/Defender/Blueprints/BP_AnimatedDialogueActor.BP_AnimatedDialogueActor_C"))
      (bind _output_get (Variables|Default|SetAnimatedDialofueActor (Utilities|Array|Get(acopy) _outactors)))
      (Utilities|IsValid _output_get
        (:Is%20Valid
          (EventDispatchers|AssignOnDialogueEventTriggered (Variables|Default|GetAnimatedDialofueActor) (delegate Custom|GiveQuest))
          (bind _outactors_2 (Actor|GetAllActorsOfClass "/Game/Defender/Blueprints/BP_AnimatedDialogueActor.BP_AnimatedDialogueActor_C"))
          (Variables|Default|SetDialogueWb (Default|GetDialogueScreenWidget (Utilities|Array|Get(acopy) _outactors_2))))
        (:Is%20Not%20Valid
          (Development|PrintString "ERROR: Animated Dialogue Actor is not found on level" true true "(R=1.000000,G=0.008304,B=0.000000,A=1.000000)" 4.0))))
    (:Is%20Not%20Valid
      (Development|PrintString "ERROR: No interactor component found in character" true true "(R=1.000000,G=0.006324,B=0.000000,A=1.000000)" 5.0))))

(event EventTick
  (params (DeltaSeconds :type Float%20%28single-precision%29))
  (bind _timerhandle (Variables|Default|GetTimerHandle))
  (if (Widget|IsVisible (Variables|Default|GetDialogueWb))
    (Utilities|Time|PauseTimerbyHandle _timerhandle)
    (else
      (Utilities|Time|UnpauseTimerbyHandle _timerhandle))))

(fn AddNewQuest
  (params (QuestID :type Name))
  (bind _returnvalue (Class|DataTableFunctionLibrary|DoesDataTableRowExist "/Game/Defender/Datatables/QuestTables/DT_GameplayQuests.DT_GameplayQuests" QuestID))
  (if _returnvalue
    (if (and (== (Utilities|Array|FindItem (Variables|Default|GetCompletedQuests) QuestID) -1) (== (Utilities|Array|FindItem (Variables|Default|GetCurrentActiveQuests) QuestID) -1))
      (Utilities|Array|AddUnique (Variables|Default|GetCurrentActiveQuests) QuestID)
      (bind _returnvalue_2 (Game|SpawnActorfromClass "/Game/Defender/Blueprints/Quest/BP_QuestParent.BP_QuestParent_C" (Math|Transform|MakeTransform "0, 0, 0" "0, 0, 0" "1.000000,1.000000,1.000000") "AdjustIfPossibleButAlwaysSpawn" "OverrideRootScale" 0 QuestID self 0))
      (Utilities|Array|Add (Variables|Default|GetCurrentQuests) _returnvalue_2))))

(fn CompeleQuest
  (params (QuestID :type Name%20%28by%20ref%29))
  (Utilities|Array|AddUnique (Variables|Default|GetCompletedQuests) QuestID)
  (Utilities|Array|RemoveItem (Variables|Default|GetCurrentActiveQuests) QuestID)
  (bind _questactor (CallFunction|GetQuestActor QuestID))
  (Default|ShowImportantMessage (Variables|Default|GetAnimatedDialofueActor) (Variables|/Game/Defender/Blueprints/DataAssets/PD_QuestDataAsset.PD_QuestDataAsset_C|GetQuestName (Variables|/Game/Defender/Blueprints/Quest/BP_QuestParent.BP_QuestParent_C|GetQuest%20DA _questactor)) "NewEnumerator0")
  (bind _questactor_2 (CallFunction|GetQuestActor QuestID))
  (Default|CallOnQuestCompleted _questactor_2))

(fn QueryActiveQuest
  (params (QuestID :type Name))
  (return (Utilities|Array|ContainsItem (Variables|Default|GetCurrentActiveQuests) QuestID)))

(fn TrackQuest)

(fn TurninQuest
  (params (QuestID :type Name) (IsSuccesful :type Boolean))
  (bind _returnvalue (Game|GetPlayerCharacter 0))
  (bind _returnvalue_2 (Game|GetPlayerCharacter 0))
  (bind _returnvalue_3 (Actor|GetComponentbyClass _returnvalue "/Game/Defender/Blueprints/Components/InventoryComponent.InventoryComponent_C"))
  (bind _returnvalue_4 (Actor|GetComponentbyClass _returnvalue_2 "/Game/Defender/Blueprints/Components/InventoryComponent.InventoryComponent_C"))
  (if IsSuccesful
    (Utilities|FlowControl|Sequence
      (:then_0
        (bind _questactor (CallFunction|GetQuestActor QuestID))
        ;[0 0 0] Rewards
        (Utilities|IsValid _returnvalue_3
          (:Is%20Valid
            (LocalVariables|SetInventoryComp _returnvalue_3)
            (bind _keys (Utilities|Map|Keys (.Rewards (Utilities|Struct|BreakQuestStageStruct (Variables|/Game/Defender/Blueprints/Quest/BP_QuestParent.BP_QuestParent_C|GetCurrentStageDetails _questactor)))))
            (for _array_element _keys
              (bind _output_get (LocalVariables|SetCurrentItemName (Utilities|String|ToString(Name) _array_element)))
              (bind _isjustitem (CallFunction|SpecialTextTagRewardEvents _output_get))
              (if (and (not (Utilities|String|Contains (LocalVariables|GetCurrentItemName) "FailReward")) _isjustitem)
                (Default|AddtoInventory (LocalVariables|GetInventoryComp) (Utilities|String|StringToName (LocalVariables|GetCurrentItemName)) (.Value (Utilities|Map|Find (.Rewards (Utilities|Struct|BreakQuestStageStruct (Variables|/Game/Defender/Blueprints/Quest/BP_QuestParent.BP_QuestParent_C|GetCurrentStageDetails _questactor))) _array_element))))))))
      (:then_1
        (bind _questactor_2 (CallFunction|GetQuestActor QuestID))
        (if (Variables|/Game/Defender/Blueprints/Quest/BP_QuestParent.BP_QuestParent_C|GetIsComplete _questactor_2)
          (CallFunction|CompeleQuest QuestID))))
    (else
      (Utilities|FlowControl|Sequence
        (:then_0
          (bind _questactor_3 (CallFunction|GetQuestActor QuestID))
          ;[0 0 0] Rewards
          (Utilities|IsValid _returnvalue_4
            (:Is%20Valid
              (LocalVariables|SetInventoryComp _returnvalue_4)
              (bind _keys_2 (Utilities|Map|Keys (.Rewards (Utilities|Struct|BreakQuestStageStruct (Variables|/Game/Defender/Blueprints/Quest/BP_QuestParent.BP_QuestParent_C|GetCurrentStageDetails _questactor_3)))))
              (for _array_element_2 _keys_2
                (LocalVariables|SetCurrentItemName (Utilities|String|ToString(Name) _array_element_2))
                (if (Utilities|String|Contains (LocalVariables|GetCurrentItemName) "FailReward")
                  (bind _output_get_2 (LocalVariables|SetCurrentItemName (Utilities|String|Replace (LocalVariables|GetCurrentItemName) "FailReward")))
                  (bind _isjustitem_2 (CallFunction|SpecialTextTagRewardEvents _output_get_2))
                  (if _isjustitem_2
                    (Default|AddtoInventory (LocalVariables|GetInventoryComp) (Utilities|String|StringToName (LocalVariables|GetCurrentItemName)) (.Value (Utilities|Map|Find (.Rewards (Utilities|Struct|BreakQuestStageStruct (Variables|/Game/Defender/Blueprints/Quest/BP_QuestParent.BP_QuestParent_C|GetCurrentStageDetails _questactor_3))) _array_element_2)))))))))
        (:then_1
          (CallFunction|FailQuest QuestID))))))

(fn GetQuestActor
  (params (QuestID :type Name))
  (for _array_element (Variables|Default|GetCurrentQuests)
    (if (== QuestID (Variables|/Game/Defender/Blueprints/Quest/BP_QuestParent.BP_QuestParent_C|GetQuestID _array_element))
      (return _array_element))))

(fn FailQuest
  (params (QuestID :type Name%20%28by%20ref%29))
  (Utilities|Array|AddUnique (Variables|Default|GetCompletedQuests) QuestID)
  (Utilities|Array|RemoveItem (Variables|Default|GetCurrentActiveQuests) QuestID)
  (bind _questactor (CallFunction|GetQuestActor QuestID))
  (Default|ShowImportantMessage (Variables|Default|GetAnimatedDialofueActor) (Variables|/Game/Defender/Blueprints/DataAssets/PD_QuestDataAsset.PD_QuestDataAsset_C|GetQuestName (Variables|/Game/Defender/Blueprints/Quest/BP_QuestParent.BP_QuestParent_C|GetQuest%20DA _questactor)) "NewEnumerator1")
  (bind _questactor_2 (CallFunction|GetQuestActor QuestID))
  (Default|CallOnQuestCompleted _questactor_2))

(fn SpecialTextTagRewardEvents
  (params (CurrentRewardText :type String))
  (if (Utilities|String|Contains CurrentRewardText "NextQuest")
    (CallFunction|AddNewQuest (Utilities|String|StringToName (Utilities|String|Replace CurrentRewardText "NextQuest")))
    (return false)
    (elif (Utilities|String|Contains CurrentRewardText "ExecuteEvent")
      (Default|CallOnDialogueEventTriggered (Variables|Default|GetAnimatedDialofueActor) (Utilities|String|StringToName (Utilities|String|Replace CurrentRewardText "ExecuteEvent")))
      (return false)
      (else
        (return true)))))

(fn AutoQuestandEventGamemodeTimer
  (Utilities|FlowControl|Sequence
    (:then_0
      (if (Variables|Quest|GetIsFirstTick)
        (Variables|Quest|SetIsFirstTick false)
        (bind _outrownames (DataTable|GetDataTableRowNames "/Game/Defender/Datatables/QuestTables/DT_GameplayQuests.DT_GameplayQuests"))
        (bind _output_get (LocalVariables|SetQuestArray _outrownames))
        (for _array_element _output_get
          (bind _returnvalue (Utilities|GetDataTableRow "/Game/Defender/Datatables/QuestTables/DT_GameplayQuests.DT_GameplayQuests" _array_element)
            (:then
              (if (and (>= (.Minutes (Utilities|Struct|BreakGameplayTimeStruct (.AutoQuestTime (Utilities|Struct|BreakAllGameQuestsStruct _returnvalue)))) 0) (>= (.Seconds (Utilities|Struct|BreakGameplayTimeStruct (.AutoQuestTime (Utilities|Struct|BreakAllGameQuestsStruct _returnvalue)))) 0))
                (Utilities|Map|Add (Variables|Quest|GetAllAutoQuest) _array_element (+ (* (.Minutes (Utilities|Struct|BreakGameplayTimeStruct (.AutoQuestTime (Utilities|Struct|BreakAllGameQuestsStruct _returnvalue)))) 60) (.Seconds (Utilities|Struct|BreakGameplayTimeStruct (.AutoQuestTime (Utilities|Struct|BreakAllGameQuestsStruct _returnvalue))))))
                (Utilities|Array|AddUnique (Variables|Quest|GetQuestsTimes) (+ (* (.Minutes (Utilities|Struct|BreakGameplayTimeStruct (.AutoQuestTime (Utilities|Struct|BreakAllGameQuestsStruct _returnvalue)))) 60) (.Seconds (Utilities|Struct|BreakGameplayTimeStruct (.AutoQuestTime (Utilities|Struct|BreakAllGameQuestsStruct _returnvalue))))))
                (if (< (+ (* (.Minutes (Utilities|Struct|BreakGameplayTimeStruct (.AutoQuestTime (Utilities|Struct|BreakAllGameQuestsStruct _returnvalue)))) 60) (.Seconds (Utilities|Struct|BreakGameplayTimeStruct (.AutoQuestTime (Utilities|Struct|BreakAllGameQuestsStruct _returnvalue))))) (LocalVariables|GetNextAutoquestQuestTime))
                  (LocalVariables|SetNextAutoquestQuestID _array_element)
                  (LocalVariables|SetNextAutoquestQuestTime (+ (* (.Minutes (Utilities|Struct|BreakGameplayTimeStruct (.AutoQuestTime (Utilities|Struct|BreakAllGameQuestsStruct _returnvalue)))) 60) (.Seconds (Utilities|Struct|BreakGameplayTimeStruct (.AutoQuestTime (Utilities|Struct|BreakAllGameQuestsStruct _returnvalue)))))))))))
        (bind _outrownames_2 (DataTable|GetDataTableRowNames "/Game/Defender/Datatables/QuestTables/DT_GameplayEvents.DT_GameplayEvents"))
        (for _array_element_2 _outrownames_2
          (bind _returnvalue_2 (Utilities|GetDataTableRow "/Game/Defender/Datatables/QuestTables/DT_GameplayEvents.DT_GameplayEvents" _array_element_2)
            (:then
              (Utilities|Map|Add (Variables|Quest|GetAllAutoEvents) _array_element_2 (+ (* (.minutes (.eventtime _returnvalue_2)) 60) (.seconds (.eventtime _returnvalue_2))))
              (Utilities|Array|AddUnique (Variables|Quest|GetEventTimes) (+ (* (.minutes (.eventtime _returnvalue_2)) 60) (.seconds (.eventtime _returnvalue_2))))
              (if (< (+ (* (.minutes (.eventtime _returnvalue_2)) 60) (.seconds (.eventtime _returnvalue_2))) (LocalVariables|GetNextAutoEventTime))
                (LocalVariables|SetNextAutoEventName _array_element_2)
                (LocalVariables|SetNextAutoEventTime (+ (* (.minutes (.eventtime _returnvalue_2)) 60) (.seconds (.eventtime _returnvalue_2))))))))))
    (:then_1
      (bind _result (Math|Integer|IncrementInt (Variables|Quest|GetGamemodeTimer))
        (:%20%20
          (Utilities|FlowControl|Sequence
            (:then_0
              (if (!= (Utilities|Array|FindItem (Variables|Quest|GetQuestsTimes) _result) -1)
                (bind _keys (Utilities|Map|Keys (Variables|Quest|GetAllAutoQuest)))
                (for _array_element_3 _keys
                  (if (== (.Value (Utilities|Map|Find (Variables|Quest|GetAllAutoQuest) _array_element_3)) (Variables|Quest|GetGamemodeTimer))
                    (CallFunction|AddNewQuest _array_element_3)))))
            (:then_1
              (if (!= (Utilities|Array|FindItem (Variables|Quest|GetEventTimes) _result) -1)
                (bind _keys_2 (Utilities|Map|Keys (Variables|Quest|GetAllAutoEvents)))
                (for _array_element_4 _keys_2
                  (if (== (.Value (Utilities|Map|Find (Variables|Quest|GetAllAutoEvents) _array_element_4)) (Variables|Quest|GetGamemodeTimer))
                    (Default|CallOnDialogueEventTriggered (Variables|Default|GetAnimatedDialofueActor) _array_element_4)))))))))))