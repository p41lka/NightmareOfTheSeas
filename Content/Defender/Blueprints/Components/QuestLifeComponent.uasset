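; Quest component that reports its owning actor's destruction to the player's interactor component, apparently for quest progress.
; On BeginPlay it caches the InteractorComp from player character 0 and binds to the owner's OnDestroyed event, printing an error if none is found.
; When the owner is destroyed, it calls ObjectIDPassed on that interactor with its ObjectID and a value of one.
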(event Custom|OnOwnerDestroyed
  (params (DestroyedActor :type Actor%20Object%20Reference))
  (Default|CallObjectIDPassed (Variables|Default|GetInteractorConponent) (Variables|Default|GetObjectID) 1))

(event EventBeginPlay
  (bind _returnvalue (Game|GetPlayerCharacter 0))
  (bind _returnvalue_2 (Actor|GetComponentbyClass _returnvalue "/Game/Defender/Blueprints/Components/InteractorComp.InteractorComp_C"))
  (Utilities|IsValid _returnvalue_2
    (:Is%20Valid
      (Variables|Default|SetInteractorConponent _returnvalue_2)
      (Game|AssignOnDestroyed (Components|GetOwner) (delegate Custom|OnOwnerDestroyed)))
    (:Is%20Not%20Valid
      (Development|PrintString "ERROR: No interactor component found in character" true true "(R=1.000000,G=0.006324,B=0.000000,A=1.000000)" 5.0))))

(event EventTick
  (params (DeltaSeconds :type Float%20%28single-precision%29)))