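; Inventory component that stores item counts in a map, capped at three items in total across all types.
; AddToInventory handles additions and removals, deleting emptied entries, and passes changes that leave a positive count to player character 0's interactor component, cached at BeginPlay.
; DropItem looks up the actor class in DT_GameplayItems, spawns it ahead of the owner and decrements through AddToInventory.
; QueryInventory returns an item's count.
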(event EventBeginPlay
  (bind _returnvalue (Game|GetPlayerCharacter 0))
  (bind _returnvalue_2 (Actor|GetComponentbyClass _returnvalue "/Game/Defender/Blueprints/Components/InteractorComp.InteractorComp_C"))
  (Utilities|IsValid _returnvalue_2
    (:Is%20Valid
      (Variables|Default|SetInteractorConponent _returnvalue_2))
    (:Is%20Not%20Valid
      (Development|PrintString "ERROR: No interactor component found in character" true true "(R=1.000000,G=0.006324,B=0.000000,A=1.000000)" 5.0))))

(event EventTick
  (params (DeltaSeconds :type Float%20%28single-precision%29)))

(fn AddtoInventory
  (params (Item :type Name) (Quantity :type Integer))
  (bind _content (Variables|Default|GetContent))
  (bind _content_2 (Variables|Default|GetContent))
  (bind _value (Utilities|Map|Find _content_2 Item))
  (bind _returnvalue (+ Quantity _value))
  (Variables|Default|SetItemNumber 0)
  (bind _keys (Utilities|Map|Keys _content))
  (for _array_element _keys
    (Variables|Default|SetItemNumber (+ (.Value (Utilities|Map|Find _content _array_element)) (Variables|Default|GetItemNumber))))
  (if (> (+ (Variables|Default|GetItemNumber) Quantity) 3)
    (return false)
    (elif (> _returnvalue 0)
      (Utilities|Map|Add (Variables|Default|GetContent) Item _returnvalue)
      (Default|CallObjectIDPassed (Variables|Default|GetInteractorConponent) Item Quantity)
      (return true)
      (else
        (Utilities|Map|Remove (Variables|Default|GetContent) Item)
        (return true)))))

(fn QueryInventory
  (params (Item :type Name))
  (return (.Value (Utilities|Map|Find (Variables|Default|GetContent) Item))))

(fn DropItem
  (params (ItemName :type Name))
  (bind _returnvalue (Components|GetOwner))
  (bind _returnvalue_2 (Utilities|GetDataTableRow "/Game/Defender/Datatables/QuestTables/DT_GameplayItems.DT_GameplayItems" ItemName)
    (:then
      (if (> (.Value (Utilities|Map|Find (Variables|Default|GetContent) ItemName)) 0)
        (Game|SpawnActorfromClass (.ActorClass (Utilities|Struct|BreakItemDescriptionStruct _returnvalue_2)) (Math|Conversions|ToTransform(Vector) (+ (* (Transformation|GetActorForwardVector _returnvalue) "100.000000,100.000000,100.000000") (Transformation|GetActorLocation _returnvalue))) "AdjustIfPossibleButAlwaysSpawn" "SelectDefaultAtRuntime" 0 0)
        (CallFunction|AddtoInventory ItemName -1)))))