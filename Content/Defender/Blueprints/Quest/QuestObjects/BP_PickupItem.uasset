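; BP_PickupItem is a world pickup in the quest objects folder that gives an item to the player.
; When its sphere is overlapped by an actor of the player character's class, it finds the InventoryComponent on player 0's character and adds ItemName with Quantity, then destroys itself.
; If that component is missing, it prints an error and stays in the world.
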(event OnComponentBeginOverlap(Sphere)
  (params (OverlappedComponent :type Primitive%20Component%20Object%20Reference) (OtherActor :type Actor%20Object%20Reference) (OtherComp :type Primitive%20Component%20Object%20Reference) (OtherBodyIndex :type Integer) (bFromSweep :type Boolean) (SweepResult :type Hit%20Result%20Structure%20%28by%20ref%29))
  (bind _returnvalue (Game|GetPlayerCharacter 0))
  (bind _returnvalue_2 (Actor|GetComponentbyClass _returnvalue "/Game/Defender/Blueprints/Components/InventoryComponent.InventoryComponent_C"))
  (if (== (Utilities|GetClass OtherActor) (Utilities|GetClass _returnvalue))
    (Utilities|IsValid _returnvalue_2
      (:Is%20Valid
        (bind _output_get (Variables|Default|SetInventoryComponent _returnvalue_2))
        (Default|AddtoInventory _output_get (Variables|Default|GetItemName) (Variables|Default|GetQuantity))
        (Actor|DestroyActor))
      (:Is%20Not%20Valid
        (Development|PrintString "ERROR: Inventory component not found in player")))))

(event EventBeginPlay)

(fn ConstructionScript)