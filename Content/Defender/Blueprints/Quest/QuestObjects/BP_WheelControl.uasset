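; BP_WheelControl is an interactable quest-object control that changes how fast a linked environment object rotates.
; Each InteractionPressed call raises or lowers EnvirMov's RotSpeed by a fixed step, with the RightOrLeft flag choosing the direction.
; The new speed is written to a single axis of that object's RotatingMovement rotation rate, with no clamp, and a debug "Hello" is printed.
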(event EventBeginPlay
  (|CallParentFunction) ; This node is disabled and will not be called.\nDrag off pins to build functionality.
)

(event Collision|EventActorBeginOverlap
  (params (OtherActor :type Actor%20Object%20Reference))
  (|CallParentFunction OtherActor) ; This node is disabled and will not be called.\nDrag off pins to build functionality.
)

(event EventTick
  (params (DeltaSeconds :type Float%20%28single-precision%29))
  (|CallParentFunction DeltaSeconds) ; This node is disabled and will not be called.\nDrag off pins to build functionality.
)

(fn ConstructionScript
  (|CallParentFunction))

(fn InteractionPressed
  (params (Interactor :type Actor%20Object%20Reference))
  (bind _envirmov (Variables|Default|GetEnvirMov))
  (bind _output_get (Variables|/Game/Blueprints/MiniGames/Levi/BP_EviromentMovement.BP_EviromentMovement_C|SetRotSpeed _envirmov (+ (Variables|/Game/Blueprints/MiniGames/Levi/BP_EviromentMovement.BP_EviromentMovement_C|GetRotSpeed _envirmov) (Math|Float|SelectFloat 2.0 -2.0 (Variables|Default|GetRightOrLeft)))))
  (Variables|/Script/Engine.RotatingMovementComponent|SetRotationRate (Variables|/Game/Blueprints/MiniGames/Levi/BP_EviromentMovement.BP_EviromentMovement_C|GetRotatingMovement _envirmov) (Math|Rotator|MakeRotator 0.0 0.0 _output_get))
  (Development|PrintString "Hello")
  (return "None"))